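; Procedural road network Blueprint that rebuilds stacked road layers over noise-based terrain whenever RegenerateRoads fires.
; Each layer's path comes from a seeded population-and-generations search, and FindConnectionPairs links it to the layer below with slope-limited A* ramps.
; DrawRoad turns paths into splines with spline meshes, using line traces to seat layer 0 just above the ground.
; Per-layer material code is disconnected, and DrawRoad2 is an uncalled variant.
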(event `RegenerateRoads`
  (params (NoiseScale :type "Float (double-precision)") (HeightMult :type "Float (double-precision)") (MaxSlope :type "Float (double-precision)") (Vertices :type "Array of Vector Structure") (NoiseOffsetX :type Integer) (NoiseOffsetY :type Integer) (Seed :type Integer) (Layers :type Integer))
  (set `self.NoiseScale` NoiseScale)
  (set `self.HeigthMult` HeightMult)
  (set `self.MaxSlope` MaxSlope)
  (set `self.OffsetX` NoiseOffsetX)
  (set `self.OffsetY` NoiseOffsetY)
  (set `self.Seed` Seed)
  (set `self.NrLayers` Layers)
  (`self.ClearRoads`)
  (for _index (range (+ (`self.NrLayers`) 1))
    (bind _returnvalue (`RoadGenLib.GenerateSingleRoadFromVertices` (+ _index (`self.Seed`)) Vertices true 30 40 6 (`self.NoiseScale`) (`self.HeigthMult`) (`self.MaxSlope`) _index (`self.OffsetX`) (`self.OffsetY`)))
    (bind _returnvalue_2 (`AddComponent|NODE_AddSplineComponent-5` :`bManualAttachment` true))
    (`SplineComponent.ClearSplinePoints` _returnvalue_2 true)
    (`self.DrawRoad` (- (`KismetArrayLibrary.Array_Length` (break `RoadPath` _returnvalue)) 2) _returnvalue_2 (break `RoadPath` _returnvalue) (`.Layer` (break `RoadPath` _returnvalue)))
    (`KismetSystemLibrary.PrintString` "Wygenerowano wartwę" true true (struct :`G` 0.66 :`B` 0.446957 :`A` 1.0))
    (if (== (`.Layer` (break `RoadPath` _returnvalue)) 0)
      (bind _roadpath (make `RoadPath` (break `RoadPath` _returnvalue) (`.Fitness` (break `RoadPath` _returnvalue)) (`.Layer` (break `RoadPath` _returnvalue))))
      (set `self.PreviousLayerRoad` _roadpath)
      (else
        (bind _returnvalue_3 (`RoadGenLib.FindConnectionPairs` (`self.PreviousLayerRoad`) _roadpath 4 (`self.MaxSlope`)))
        (set `self.PreviousLayerRoad` _roadpath)
        (for _array_element _returnvalue_3
          (bind _returnvalue_4 (`RoadGenLib.GenerateRampWithAStar` _array_element 50.0 (`self.MaxSlope`) (`self.NoiseScale`) (`self.HeigthMult`) 100000.0 (`self.OffsetX`) (`self.OffsetY`)))
          (bind _returnvalue_5 (`AddComponent|NODE_AddSplineComponent-9` :`bManualAttachment` true))
          (`SplineComponent.ClearSplinePoints` _returnvalue_5 true)
          (`self.DrawRoad` (- (`KismetArrayLibrary.Array_Length` (break `RoadPath` _returnvalue_4)) 2) _returnvalue_5 (break `RoadPath` _returnvalue_4) 99))))))

(fn `ClearRoads`
  (for _ (range 11)
    (for _array_element (`self.K2_GetComponentsByClass` "/Script/Engine.SplineMeshComponent")
      (`ActorComponent.K2_DestroyComponent` _array_element))
    (for _array_element_2 (`self.K2_GetComponentsByClass` "/Script/Engine.SplineComponent")
      (`SplineComponent.ClearSplinePoints` _array_element_2 true))))

(fn `DrawRoad`
  (params (EndIndex :type Integer) (SplineComponent :type "SplineComponent Object Reference") (TPoints :type "Array of Vector Structure") (Layer :type Integer))
  (for _index (range (+ EndIndex 1))
    (if (== Layer 0)
      (bind (_output_x _output_y _output_z) (`KismetMathLibrary.BreakVector` (`|GetArrayItem` TPoints _index)))
      (bind _outhit (`KismetSystemLibrary.LineTraceSingle` (`KismetMathLibrary.MakeVector` _output_x _output_y 1000.0) (`KismetMathLibrary.MakeVector` _output_x _output_y -1000.0) "TraceTypeQuery1"))
      (bind (_output_x_2 _output_y_2 _output_z_2) (`KismetMathLibrary.BreakVector` (`|GetArrayItem` TPoints (+ _index 1))))
      (bind _outhit_2 (`KismetSystemLibrary.LineTraceSingle` (`KismetMathLibrary.MakeVector` _output_x_2 _output_y_2 1000.0) (`KismetMathLibrary.MakeVector` _output_x_2 _output_y_2 -1000.0) "TraceTypeQuery1"))
      (`SplineComponent.AddSplinePoint` SplineComponent (`KismetMathLibrary.MakeVector` _output_x _output_y (+ (.z (`.Location` (`GameplayStatics.BreakHitResult` _outhit))) 30.0)) "World" true)
      (`SplineComponent.AddSplinePoint` SplineComponent (`KismetMathLibrary.MakeVector` _output_x_2 _output_y_2 (+ (.z (`.Location` (`GameplayStatics.BreakHitResult` _outhit_2))) 30.0)) "World" true)
      (else
        (`SplineComponent.AddSplinePoint` SplineComponent (`KismetMathLibrary.MakeVector` _output_x _output_y (+ _output_z 0.0)) "World" true)
        (`SplineComponent.AddSplinePoint` SplineComponent (`KismetMathLibrary.MakeVector` _output_x _output_y (+ _output_z_2 0.0)) "World" true))))
  (for _index_2 (range (+ (- (`SplineComponent.GetNumberOfSplinePoints` SplineComponent) 2) 1))
    (bind _returnvalue (`AddComponent|NODE_AddSplineMeshComponent-1` :`bManualAttachment` true))
    (`StaticMeshComponent.SetStaticMesh` _returnvalue (`self.RoadMesh`))
    (`SplineMeshComponent.SetStartAndEnd` _returnvalue (`SplineComponent.GetLocationAtSplinePoint` SplineComponent _index_2 "World") (`SplineComponent.GetTangentAtSplinePoint` SplineComponent _index_2 "World") (`SplineComponent.GetLocationAtSplinePoint` SplineComponent (+ _index_2 1) "World") (`SplineComponent.GetTangentAtSplinePoint` SplineComponent (+ _index_2 1) "World") true)))

(fn `DrawRoad_2`
  (params (EndIndex :type Integer) (SplineComponent :type "SplineComponent Object Reference") (TPoints :type "Array of Vector Structure") (Layer :type Integer))
  (for _index (range (+ EndIndex 1))
    (if (== Layer 0)
      (bind _output (`|GetArrayItem` TPoints _index))
      (bind _out (`self.LiftRoadLayer0` _output))
      (bind _output_2 (`|GetArrayItem` TPoints (+ _index 1)))
      (bind _out_2 (`self.LiftRoadLayer0` _output_2))
      (`SplineComponent.AddSplinePoint` SplineComponent _out "World" true)
      (`SplineComponent.AddSplinePoint` SplineComponent _out_2 "World" true)
      (else
        (`SplineComponent.AddSplinePoint` SplineComponent _output "World" true)
        (`SplineComponent.AddSplinePoint` SplineComponent _output_2 "World" true))))
  (for _index_2 (range (+ (- (`SplineComponent.GetNumberOfSplinePoints` SplineComponent) 2) 1))
    (bind _returnvalue (`AddComponent|NODE_AddSplineMeshComponent-5` :`bManualAttachment` true))
    (`StaticMeshComponent.SetStaticMesh` _returnvalue (`self.RoadMesh`))
    (`SplineMeshComponent.SetStartAndEnd` _returnvalue (`SplineComponent.GetLocationAtSplinePoint` SplineComponent _index_2 "World") (`SplineComponent.GetTangentAtSplinePoint` SplineComponent _index_2 "World") (`SplineComponent.GetLocationAtSplinePoint` SplineComponent (+ _index_2 1) "World") (`SplineComponent.GetTangentAtSplinePoint` SplineComponent (+ _index_2 1) "World") true)))

(fn `LiftRoadLayer0`
  (params (In :type "Vector Structure"))
  (returns (Out :type "Vector Structure"))
  (bind _x (.x In))
  (bind _y (.y In))
  (bind _outhit (`KismetSystemLibrary.LineTraceSingle` (`KismetMathLibrary.MakeVector` _x _y 1000.0) (`KismetMathLibrary.MakeVector` _x _y -1000.0) "TraceTypeQuery1"))
  (return (`KismetMathLibrary.MakeVector` (.x (`.Location` (`GameplayStatics.BreakHitResult` _outhit))) (.y (`.Location` (`GameplayStatics.BreakHitResult` _outhit))) (+ (.z (`.Location` (`GameplayStatics.BreakHitResult` _outhit))) 30.0))))

(fn `UserConstructionScript`)