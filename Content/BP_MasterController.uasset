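; Master controller that coordinates procedural world generation of terrain and an optional road network.
; On BeginPlay it possesses a spawned spectator pawn, shows WBP_UI with the mouse cursor and generates terrain from current settings.
; GenerateWorld stores new parameters and calls BP_TerrainGen.
; OnTerrainGenerated receives the vertices and has BP_RoadNetwork either rebuild roads using the stored noise, slope, seed and layer settings, or clear them.
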(event `GenerateWorld`
  (params (MS :type Integer) (NOX :type Integer) (NOY :type Integer) (S :type Integer) (NOL :type Integer) (HM :type "Float (double-precision)") (MRS :type "Float (double-precision)") (NS :type "Float (double-precision)") (bGR :type Boolean))
  (set `self.MapSize` MS)
  (set `self.NoiseOffsetX` NOX)
  (set `self.NoiseOffsetY` NOY)
  (set `self.Seed` S)
  (set `self.NumberOfLayers` NOL)
  (set `self.HeightMult` HM)
  (set `self.RoadMaxSlope` MRS)
  (set `self.NoiseScale` NS)
  (set `self.bGenerateRoads` bGR)
  (bind _returnvalue (`GameplayStatics.GetActorOfClass` "/Game/BP_TerrainGen.BP_TerrainGen_C" :!label _label))
  (`/Engine/EditorBlueprintResources/StandardMacros.IsValid` _returnvalue
    (:`Is Valid`
      (`/Game/BP_TerrainGen.GenerateTerrain` _returnvalue (`self.MapSize`) (`self.HeightMult`) (`self.NoiseScale`) (`self.NoiseOffsetX`) (`self.NoiseOffsetY`))
      (`KismetSystemLibrary.PrintString` "Terrain Generated"))
    (:`Is Not Valid`
      (`KismetSystemLibrary.PrintString` "ERROR: Getting Actor of Class BP_TerrainGen"))))

(event `self.ReceiveBeginPlay`
  (bind _returnvalue (`GameplayStatics.GetPlayerController` 0))
  (bind _returnvalue_2 (`|SpawnActorFromClass` "/Script/Engine.SpectatorPawn" (`KismetMathLibrary.MakeTransform` (0.0 0.0 1000.0)) "Undefined" "MultiplyWithRoot" null null))
  (`Controller.Possess` _returnvalue _returnvalue_2)
  (bind _returnvalue_3 (`|CreateWidget` "/Game/WBP_UI.WBP_UI_C"))
  (`UserWidget.AddToViewport` _returnvalue_3 0)
  (set `PlayerController.bShowMouseCursor` true _returnvalue)
  (goto _label))

(event `OnTerrainGenerated`
  (params (Vertices :type "Array of Vector Structure"))
  (bind _returnvalue (`GameplayStatics.GetActorOfClass` "/Game/BP_RoadNetwork.BP_RoadNetwork_C"))
  (`/Engine/EditorBlueprintResources/StandardMacros.IsValid` _returnvalue
    (:`Is Valid`
      (if (`self.bGenerateRoads`)
        (`/Game/BP_RoadNetwork.RegenerateRoads` _returnvalue (`self.NoiseScale`) (`self.HeightMult`) (`self.RoadMaxSlope`) Vertices (`self.NoiseOffsetX`) (`self.NoiseOffsetY`) (`self.Seed`) (`self.NumberOfLayers`))
        (`KismetSystemLibrary.PrintString` "Roads Generated")
        (else
          (`/Game/BP_RoadNetwork.ClearRoads` _returnvalue))))
    (:`Is Not Valid`
      (`KismetSystemLibrary.PrintString` "ERROR: Getting Actor of Class BP_RoadNetwork"))))

(fn `UserConstructionScript`)