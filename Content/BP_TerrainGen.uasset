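; Procedural terrain generator actor that builds a square grid mesh with collision from map size, height multiplier, noise scale and noise offsets.
; GenerateTerrain clears previous data, then CreateVertices samples noise-based GetHeight, clamps it and fills positions and UVs.
; CreateTraingles indexes two triangles per grid cell, using a running Vertex counter that is never reset here.
; Calculated normals and tangents complete the material-assigned mesh section, and vertices are passed to BP_MasterController via OnTerrainGenerated.
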(event `GenerateTerrain`
  (params (MapSize :type Integer) (HeigthMult :type "Float (double-precision)") (NoiseScale :type "Float (double-precision)") (NoiseOffsetX :type Integer) (NoiseOffsetY :type Integer))
  (`ProceduralMeshComponent.ClearAllMeshSections` (`self.ProceduralMesh`))
  (`KismetArrayLibrary.Array_Clear` (`self.Vertices`))
  (`KismetArrayLibrary.Array_Clear` (`self.Triangles`))
  (`KismetArrayLibrary.Array_Clear` (`self.UV0`))
  (`KismetArrayLibrary.Array_Clear` (`self.Normals`))
  (`KismetArrayLibrary.Array_Clear` (`self.Tangents`))
  (set `self.ZScale` HeigthMult)
  (set `self.XSize` MapSize)
  (set `self.YSize` MapSize)
  (`self.CreateVertices` NoiseScale (`self.Vertices`) NoiseOffsetX NoiseOffsetY)
  (`self.CreateTraingles`)
  (bind (_normals _tangents) (`KismetProceduralMeshLibrary.CalculateTangentsForMesh` (`self.Vertices`) (`self.Triangles`) (`self.UV0`)))
  (set `self.Normals` _normals)
  (set `self.Tangents` _tangents)
  (`ProceduralMeshComponent.CreateMeshSection_LinearColor` :`self` (`self.ProceduralMesh`) :`Vertices` (`self.Vertices`) :`Triangles` (`self.Triangles`) :`Normals` (`self.Normals`) :`UV0` (`self.UV0`) :`Tangents` (`self.Tangents`) :`bCreateCollision` true)
  (`PrimitiveComponent.SetMaterial` (`self.ProceduralMesh`) 0 (`self.Material`))
  (bind _returnvalue (`GameplayStatics.GetActorOfClass` "/Game/BP_MasterController.BP_MasterController_C"))
  (`/Game/BP_MasterController.OnTerrainGenerated` _returnvalue (`self.Vertices`)))

(fn `CreateTraingles`
  (locals (Vertex :type Integer))
  (for _ (range (`self.XSize`))
    (for _ (range (`self.YSize`))
      (`KismetArrayLibrary.Array_Add` (`self.Triangles`) (`local.Vertex`))
      (`KismetArrayLibrary.Array_Add` (`self.Triangles`) (+ (`local.Vertex`) 1))
      (`KismetArrayLibrary.Array_Add` (`self.Triangles`) (+ (`self.YSize`) (`local.Vertex`) 1))
      (`KismetArrayLibrary.Array_Add` (`self.Triangles`) (+ (`local.Vertex`) 1))
      (`KismetArrayLibrary.Array_Add` (`self.Triangles`) (+ (`self.YSize`) (`local.Vertex`) 2))
      (`KismetArrayLibrary.Array_Add` (`self.Triangles`) (+ (`self.YSize`) (`local.Vertex`) 1))
      (`/Engine/EditorBlueprintResources/StandardMacros.IncrementInt` (`local.Vertex`)))
    (`/Engine/EditorBlueprintResources/StandardMacros.IncrementInt` (`local.Vertex`))))

(fn `CreateVertices`
  (params (`Noise Scale` :type "Float (double-precision)") (GVertices :type "Array of Vector Structure") (NoiseOffsetX :type Integer) (NoiseOffsetY :type Integer))
  (locals (X :type Integer) (Y :type Integer))
  (for _index (range (+ (`self.XSize`) 1))
    (set `local.X` _index)
    (for _index_2 (range (+ (`self.YSize`) 1))
      (set `local.Y` _index_2)
      (`KismetArrayLibrary.Array_Add` GVertices (`KismetMathLibrary.MakeVector` (* (`local.X`) (`self.Scale`)) (* (`local.Y`) (`self.Scale`)) (`KismetMathLibrary.FClamp` (`PerlinNoise2D.GetHeight` (`KismetMathLibrary.Conv_IntToDouble` (`local.X`)) (`KismetMathLibrary.Conv_IntToDouble` (`local.Y`)) `Noise Scale` (`self.ZScale`) NoiseOffsetX NoiseOffsetY) (`self.ZMin`) (`self.ZScale`))))
      (`KismetArrayLibrary.Array_Add` (`self.UV0`) (`KismetMathLibrary.MakeVector2D` (* (`local.X`) (`self.UVScale`)) (* (`local.Y`) (`self.UVScale`)))))))

(fn `UserConstructionScript`)